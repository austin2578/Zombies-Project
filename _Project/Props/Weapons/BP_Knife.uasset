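; BP_Knife is a knife weapon actor that deals a single heavy stab to a BP_Zombie.
; When its Capsule begins an overlap while CanHit is true, it destroys the Capsule before casting the other actor to BP_Zombie.
; A successful cast applies fixed damage, plays a 2D impact sound and clears CanHit.
; Any overlapping actor, zombie or not, therefore uses up the hitbox.
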(event OnComponentBeginOverlap(Capsule)
  (params (OverlappedComponent :type Primitive%20Component%20Object%20Reference) (OtherActor :type Actor%20Object%20Reference) (OtherComp :type Primitive%20Component%20Object%20Reference) (OtherBodyIndex :type Integer) (bFromSweep :type Boolean) (SweepResult :type Hit%20Result%20Structure%20%28by%20ref%29))
  ;[1 1 1] Stabbing action
  (if (Variables|Default|GetCan%20Hit)
    (Components|DestroyComponent (Variables|Default|GetCapsule))
    (bind _asbp_zombie (Utilities|Casting|CastToBP_Zombie OtherActor))
    (Game|Damage|ApplyDamage _asbp_zombie 1.5e+02 0 0)
    (Audio|PlaySound2D "/Game/_Project/Resources/Audio/zapsplat_impacts_body_hit_punch_or_kick_whoosh_011_90405-VEED-VEED.zapsplat_impacts_body_hit_punch_or_kick_whoosh_011_90405-VEED-VEED" 1.0 1.0 0.0 0 0)
    (Variables|Default|SetCan%20Hit false)))

(event EventBeginPlay
  (|CallParentFunction) ; This node is disabled and will not be called.\nDrag off pins to build functionality.
)

(event Collision|EventActorBeginOverlap
  (params (OtherActor :type Actor%20Object%20Reference))
  (|CallParentFunction OtherActor) ; This node is disabled and will not be called.\nDrag off pins to build functionality.
)

(event EventTick
  (params (DeltaSeconds :type Float%20%28single-precision%29))
  (|CallParentFunction DeltaSeconds) ; This node is disabled and will not be called.\nDrag off pins to build functionality.
)

(fn ConstructionScript
  (|CallParentFunction))