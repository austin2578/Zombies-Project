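; Purchasable weapon pickup for the zombie waves mode, with its WeaponInfo loaded from a data table row in the construction script.
; Its interact details supply the weapon name and price.
; Interacting charges full price, or half if the weapon is already carried and the equipped weapon's ammo isn't full, using GM_ZombieWaves points.
; Successful purchases call the character's SpawnWeapon, and the player UI animates success or failure.
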(event EventBeginPlay
  (|CallParentFunction))

(event Collision|EventActorBeginOverlap
  (params (OtherActor :type Actor%20Object%20Reference))
  (|CallParentFunction OtherActor) ; This node is disabled and will not be called.\nDrag off pins to build functionality.
)

(event EventTick
  (params (DeltaSeconds :type Float%20%28single-precision%29))
  (|CallParentFunction DeltaSeconds) ; This node is disabled and will not be called.\nDrag off pins to build functionality.
)

(event EventInteract
  (params (CharacterPickingUp :type BP%20Vivian%20Object%20Reference))
  (bind _weaponinfo (Variables|Default|GetWeaponInfo))
  (bind _currentweapon (Variables|/Game/FirstPerson/Blueprints/BP_FirstPersonCharacter.BP_FirstPersonCharacter_C|GetCurrentWeapon CharacterPickingUp))
  (bind (_weaponname _weapontype _weaponfiremode _weaponint _pickupclass _magazinesize _damage _penetration _recoilpattern _weaponfirerate _weaponpickupanim _maxammo _currentammo _ammoreserves _ammocasing _spreadmultiplier _headshotmulti _price) (Utilities|Struct|BreakWeaponInfo_S _weaponinfo))
  (bind _weaponinfo_2 (Variables|/Game/_Project/Props/Weapons/BP_WeaponMaster_.BP_WeaponMaster__C|GetWeaponInfo _currentweapon))
  (bind (_weaponname_2 _weapontype_2 _weaponfiremode_2 _weaponint_2 _pickupclass_2 _magazinesize_2 _damage_2 _penetration_2 _recoilpattern_2 _weaponfirerate_2 _weaponpickupanim_2 _maxammo_2 _currentammo_2 _ammoreserves_2) (Utilities|Struct|BreakWeaponInfo_S _weaponinfo_2))
  (bind _returnvalue (/ _price 2.0))
  ;[1 1 1] When buying a weapon, check if player has it. If player has weapon refill ammo, if not replave current weapons
  (bind _foundwidgets (Widget|GetAllWidgetsOfClass "/Game/_Project/UI/PlayerUI_W.PlayerUI_W_C" true))
  (Variables|Default|SetPlayer%20UI%20Ref (Utilities|Array|Get(acopy) _foundwidgets))
  (bind _asgm_zombie_waves (Utilities|Casting|CastToGM_ZombieWaves (Game|GetGameMode)))
  (if (or (Utilities|Enum|Equal(Enum) (.WeaponName (Utilities|Struct|BreakWeaponInfo_S (Variables|/Game/_Project/Props/Weapons/BP_WeaponMaster_.BP_WeaponMaster__C|GetWeaponInfo (Variables|/Game/FirstPerson/Blueprints/BP_FirstPersonCharacter.BP_FirstPersonCharacter_C|GetCurrentWeapon CharacterPickingUp)))) _weaponname) (Utilities|Enum|Equal(Enum) (.WeaponName (Utilities|Struct|BreakWeaponInfo_S (Variables|/Game/MetaHumans/Vivian/BP_Vivian.BP_Vivian_C|GetSecondaryWeaponInfo CharacterPickingUp))) _weaponname))
    (if (and (>= (Variables|/Game/_Project/GameMode/GM_ZombieWaves.GM_ZombieWaves_C|GetPoints _asgm_zombie_waves) _returnvalue) (not (and (== _ammoreserves_2 _maxammo_2) (== _currentammo_2 _magazinesize_2))))
      (Default|RemovePoints _asgm_zombie_waves _returnvalue)
      (Default|InteractAnim (Variables|Default|GetPlayer%20UI%20Ref) true :!label _label)
      (Default|SpawnWeapon CharacterPickingUp (Variables|Default|GetWeaponToSpawn) (Transformation|GetActorLocation) (Variables|Default|GetWeaponInfo))
      (else
        (Default|InteractAnim (Variables|Default|GetPlayer%20UI%20Ref) false :!label _label_2)))
    (elif (>= (Variables|/Game/_Project/GameMode/GM_ZombieWaves.GM_ZombieWaves_C|GetPoints _asgm_zombie_waves) _price)
      (Default|RemovePoints _asgm_zombie_waves _price)
      (goto _label)
      (else
        (goto _label_2)))))

(fn ConstructionScript
  (|CallParentFunction)
  (bind _returnvalue (Utilities|GetDataTableRow "/Game/_Project/Props/Weapons/WeaponInfo_DT.WeaponInfo_DT" (Variables|Default|GetRowName))
    (:then
      (Variables|Default|SetWeaponInfo _returnvalue))))

(fn IsInteractable?/GetDetails
  (bind _weaponinfo (Variables|Default|GetWeaponInfo))
  ;[1 1 1] Set interact details
  (return "NewEnumerator2" (Utilities|Text|ToText(String) (.weaponname _weaponinfo)) (Math|Float|Truncate (.price _weaponinfo)) 0))