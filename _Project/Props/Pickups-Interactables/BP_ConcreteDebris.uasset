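; BP_ConcreteDebris is a purchasable interactable obstacle that offers a "Clear Debris" prompt with a price and needs no power.
; Its interaction functions report the prompt details, while the ClearDebris event caches the mesh's relative start and raised end positions.
; A timeline, with play rate scaled by OpeningTime, lerps the mesh upward by OpeningZValue, then destroys the actor when finished.
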(event EventBeginPlay
  (|CallParentFunction) ; This node is disabled and will not be called.\nDrag off pins to build functionality.
)

(event Collision|EventActorBeginOverlap
  (params (OtherActor :type Actor%20Object%20Reference))
  (|CallParentFunction OtherActor) ; This node is disabled and will not be called.\nDrag off pins to build functionality.
)

(event EventTick
  (params (DeltaSeconds :type Float%20%28single-precision%29))
  (|CallParentFunction DeltaSeconds) ; This node is disabled and will not be called.\nDrag off pins to build functionality.
)

(event EventClearDebris
  (bind _pickupstaticmesh (Variables|Default|GetPickupStaticMesh))
  (bind _relativelocation (Variables|/Script/Engine.SceneComponent|GetRelativeLocation _pickupstaticmesh))
  ;[1 1 1] Lift Block and delete on completion
  (Components|Timeline|SetPlayRate (Variables|Default|GetClearing%20Timeline) (/ 1.0 (Variables|Default|GetOpening%20Time)))
  (Variables|Default|SetStart%20Location (Variables|/Script/Engine.SceneComponent|GetRelativeLocation (Variables|Default|GetPickupStaticMesh)))
  (Variables|Default|SetEnd%20Location (Math|Vector|MakeVector (.x _relativelocation) (.y _relativelocation) (+ (.z _relativelocation) (Variables|Default|GetOpening%20Z%20Value))))
  (bind _newtrack_0 (Timeline|Clearing%20Timeline PlayFromStart)
    (:Update
      (Transformation|SetRelativeLocation (Variables|Default|GetPickupStaticMesh) (Math|Vector|Lerp(Vector) (Variables|Default|GetStart%20Location) (Variables|Default|GetEnd%20Location) _newtrack_0) false false))
    (:Finished
      (Actor|DestroyActor))))

(fn ConstructionScript
  (|CallParentFunction))

(fn CanInteract?
  ;[1 1 1] Set interact text
  (return true false))

(fn IsInteractable?/GetDetails
  ;[1 1 1] Set interact text
  (return "NewEnumerator3" "Clear Debris" 1250 0))