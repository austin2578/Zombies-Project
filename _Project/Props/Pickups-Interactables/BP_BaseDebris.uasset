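; Base Blueprint for purchasable debris in the zombie waves mode, exposing price, text and interact state through interaction functions.
; Interact checks points, CanInteract and NeedPower, then plays HUD feedback, deducts the price and flags its room in the game mode's SpawnRoomsOpened.
; ClearDebris is an empty event for each debris to override.
; The NeedPower branch checks power but never clears, and insufficient points plays the failed HUD animation.
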(event Custom|Clear%20Debris
  ;[1 1 1] Event to be overridden by each debris
)

(event EventBeginPlay
  (|CallParentFunction)
  ;[1 1 1] Set interact values
  (CallFunction|CanInteract?)
  (CallFunction|IsInteractable?/GetDetails))

(event Collision|EventActorBeginOverlap
  (params (OtherActor :type Actor%20Object%20Reference))
  (|CallParentFunction OtherActor) ; This node is disabled and will not be called.\nDrag off pins to build functionality.
)

(event EventTick
  (params (DeltaSeconds :type Float%20%28single-precision%29))
  (|CallParentFunction DeltaSeconds) ; This node is disabled and will not be called.\nDrag off pins to build functionality.
)

(event EventInteract
  (params (CharacterPickingUp :type BP%20Vivian%20Object%20Reference))
  (bind _foundwidgets (Widget|GetAllWidgetsOfClass "/Game/_Project/UI/PlayerUI_W.PlayerUI_W_C" true))
  (Variables|Default|SetHUD%20Ref (Utilities|Array|Get(acopy) _foundwidgets))
  (bind _asgm_zombie_waves (Utilities|Casting|CastToGM_ZombieWaves (Game|GetGameMode)))
  (bind _output_get (Variables|Default|SetAs%20GM%20Zombie%20Waves _asgm_zombie_waves))
  ;[1 1 1] Clear Debris if player has enough points. Fail interact if failed
  (if (>= (Variables|/Game/_Project/GameMode/GM_ZombieWaves.GM_ZombieWaves_C|GetPoints _output_get) (Variables|Default|GetPrice))
    (if (Variables|Default|GetCan%20Interact)
      (if (Variables|Default|GetNeed%20Power?)
        (if (Variables|/Game/_Project/GameMode/GM_ZombieWaves.GM_ZombieWaves_C|GetIsPowerOn? _output_get)
          _)
        (else
          (Default|InteractAnim (Variables|Default|GetHUD%20Ref) true)
          (Default|RemovePoints (Variables|Default|GetAs%20GM%20Zombie%20Waves) (Math|Conversions|ToFloat(Integer) (Variables|Default|GetPrice)))
          (Utilities|Array|SetArrayElem (Variables|/Game/_Project/GameMode/GM_ZombieWaves.GM_ZombieWaves_C|GetSpawn%20Rooms%20Opened (Variables|Default|GetAs%20GM%20Zombie%20Waves)) (Variables|Default|GetRoom%20Number) true)
          (CallFunction|ClearDebris))))
    (else
      (Default|InteractAnim (Variables|Default|GetHUD%20Ref) false))))

(fn ConstructionScript
  (|CallParentFunction))

(fn CanInteract?
  ;[1 1 1] Set interact values
  (return (Variables|Default|GetCan%20Interact) (Variables|Default|GetNeed%20Power?)))

(fn IsInteractable?/GetDetails
  ;[1 1 1] Set interact details
  (return "NewEnumerator3" (Variables|Default|GetText) (Variables|Default|GetPrice) 0))