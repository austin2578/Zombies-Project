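; Game mode that runs round-based zombie waves and tracks player points with popup widgets.
; Each round derives zombie count and speeds from the round number, then a looping timer spawns zombies at random SpawnBoxes in opened rooms, limited by an alive cap.
; Remaining-quota odds mix in runners from round 4 and sprinters from 20.
; The RoundEnd dispatcher raises health, resets counters and starts the next wave after a delay.
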(event Custom|Start%20Game
  ;[1 1 1] On game start, wait 10 seconds then start zombie count loop. Bind event dispatcher Round End to EndRound event
  (Utilities|FlowControl|Delay 1e+01)
  (CallFunction|GetZombieCount)
  (EventDispatchers|BindEventtoRoundEnd (delegate Custom|EndRound)))

(event Custom|GetZombieCount
  (bind _round (Variables|Default|GetRound))
  (bind _output_get (Variables|Default|SetTotalEnemyInRound (Math|Conversions|ToFloat(Integer) (Math|Integer|SelectInt (Math|Float|Round (+ (* (Math|Float|Square (Variables|Default|GetRound)) 0.0842) (* (Variables|Default|GetRound) 0.1954) 22.05)) (Math|Integer|SelectInt (Math|Float|Round (* (* (Variables|Default|GetRound) 0.15) (Variables|Default|GetMaxEnemyInLevel))) (Math|Integer|SelectInt 7 10 (== _round 1.0)) (> _round 2.0)) (> (Variables|Default|GetRound) 11.0)))))
  (Variables|Default|SetTempZombieKills _output_get)
  ;[1 1 1] Set values of Walk/Run/Sprint for Zombies based off of round
  (CallFunction|SetMoveSpeed)
  ;[1 1 1] Set zombie swipe speed
  (CallFunction|SetAttackSpeed)
  ;[1 1 1] Time between spawns
  (Utilities|FlowControl|Delay 0.2)
  (bind _returnvalue (Utilities|Time|SetTimerbyEvent (delegate Custom|SpawnZombie) (Variables|Default|GetTimeBetweenSpawn) true)))

(event Custom|SpawnZombie
  ;[1 1 1] Event to spawn Zombie with correct speed at correct location
  ;[1 1 1] Stop spawning when spawn limit reached
  (if (< (Variables|Default|GetZombiesSpawned) (Variables|Default|GetTotalEnemyInRound))
    (if (<= (Variables|Default|GetZombiesAlive) (Variables|Default|GetMaxEnemyInLevel))
      ;[1 1 1] Set zombie speed walker/runner/sprinter
      (CallFunction|SetifWalker/Runner/Sprinter)
      ;[1 1 1] Check valid spawn locations and spawn
      (CallFunction|CheckSpawnLocationThenSpawn)
      ;[1 1 1] Increment Zombies Counters
      (Variables|Default|SetZombiesSpawned (+ (Variables|Default|GetZombiesSpawned) 1.0))
      (Variables|Default|SetZombiesAlive (+ (Variables|Default|GetZombiesAlive) 1.0)))
    (else
      (Utilities|Time|ClearandInvalidateTimerbyHandle (stale Custom|GetZombieCount _returnvalue)))))

(event Custom|EndRound
  ;[1 1 1] Commence End round, increase health and round, reset zombie counter values. Start Zombie Count loop again
  (CallFunction|IncreaseMaxHealth)
  (Variables|Default|SetRound (+ (Variables|Default|GetRound) 1.0))
  (Variables|Default|SetZombiesAlive 0.0)
  (Variables|Default|SetZombiesSpawned 0.0)
  (Variables|Default|SetRunnersSpawned 0.0)
  (Variables|Default|SetSprintersSpawned 0.0)
  (Utilities|FlowControl|Delay (Variables|Default|GetTimeBetweenRounds))
  (CallFunction|GetZombieCount))

(event EventBeginPlay
  ;[1 1 1] Commence game start
  (CallFunction|StartGame))

(event EventTick
  (params (DeltaSeconds :type Float%20%28single-precision%29)))

(fn ConstructionScript)

(fn CheckSpawnLocationThenSpawn
  (bind _maxzombiehealth (Variables|Default|GetMaxZombieHealth))
  (LocalVariables|SetSpawned? false)
  (LocalVariables|SetSpawns%20Open 0.0)
  (bind _outactors (Actor|GetAllActorsOfClass "/Game/_Project/GameMode/Spawning/SpawnBox.SpawnBox_C"))
  ;[1 1 1] Check which rooms have been opened, add those rooms to a possible spawn array
  (for _array_element _outactors
    (if (Utilities|Array|Get(acopy) (Variables|Default|GetSpawn%20Rooms%20Opened) (Variables|/Game/_Project/GameMode/Spawning/SpawnBox.SpawnBox_C|GetRoom%20Number _array_element))
      (LocalVariables|SetSpawns%20Open (+ (LocalVariables|GetSpawns%20Open) 1.0))))
  ;[1 1 1] Chance to spawn in any opened room
  (for _array_element_2 _outactors :!label _label
    (LocalVariables|SetArray%20Elem _array_element_2)
    (if (not (LocalVariables|GetSpawned?))
      (if (Utilities|Array|Get(acopy) (Variables|Default|GetSpawn%20Rooms%20Opened) (Variables|/Game/_Project/GameMode/Spawning/SpawnBox.SpawnBox_C|GetRoom%20Number (LocalVariables|GetArray%20Elem)))
        (if (<= (Math|Random|RandomFloatinRange 0.0 1.0) (/ 1.0 (LocalVariables|GetSpawns%20Open)))
          (Game|SpawnActorfromClass "/Game/_Project/Enemy/ZombieAssets/Blueprints/BP_Zombie_1.BP_Zombie_1_C" (Math|Transform|MakeTransform (Transformation|GetActorLocation (LocalVariables|GetArray%20Elem)) (Transformation|GetActorRotation (LocalVariables|GetArray%20Elem)) "1.000000,1.000000,1.000000") "AdjustIfPossibleButAlwaysSpawn" "MultiplyWithRoot" 0 _maxzombiehealth _maxzombiehealth (Variables|Default|GetZombie%20Max%20Walk%20Speed) 0)
          (LocalVariables|SetSpawned? true)))))
  (if (not (LocalVariables|GetSpawned?))
    (goto _label)))

(fn IncreaseMaxHealth
  ;[1 1 1] Calculate Zombie health based off round
  (Variables|Default|SetMaxZombieHealth (Math|Conversions|ToFloat(Integer) (Math|Integer|Clamp(Integer) (Math|Integer|SelectInt (Math|Float|Truncate (* (Variables|Default|GetMaxZombieHealth) 1.1)) (Math|Float|Truncate (+ (Variables|Default|GetMaxZombieHealth) 1e+02)) (> (Variables|Default|GetRound) 1e+01)) 150 50000))))

(fn SetAttackSpeed
  (bind _round (Variables|Default|GetRound))
  ;[1 1 1] Set Zombie Attack Speed based off round
  (Variables|Default|SetAttack%20Speed (Math|Float|Clamp(Float) (select (Math|Float|InRange(Float) _round 0.0 2e+01) (+ (* _round 0.01) 0.8) (select false (+ (* (- (Variables|Default|GetRound) 2e+01) 0.005) 1.0) 1.4)) 0.8 1.4)))

(fn SetMoveSpeed
  (bind _round (Variables|Default|GetRound))
  (bind _round_2 (Variables|Default|GetRound))
  (bind _round_3 (Variables|Default|GetRound))
  ;[1 1 1] Calculate Zombie Walk, Run, and Sprint speed
  (Variables|Default|SetWalk%20Speed (Math|Float|Clamp(Float) (select (Math|Float|InRange(Float) _round_2 0.0 2e+01) (+ (* _round_2 2.5) 3e+01) 8e+01) 3e+01 8e+01))
  (Variables|Default|SetRun%20Speed (Math|Float|Clamp(Float) (select (Math|Float|InRange(Float) _round_3 0.0 3e+01) (+ (* _round_3 6.0) 1.9e+02) 3.7e+02) 2e+02 3.7e+02))
  (Variables|Default|SetSprint%20Speed (Math|Float|Clamp(Float) (select (Math|Float|InRange(Float) _round 0.0 35.0) (+ (* _round 7.0) 3.5e+02) 4.5e+02) 3.7e+02 4.5e+02)))

(fn SetifWalker/Runner/Sprinter
  (bind _round (Variables|Default|GetRound))
  ;[1 1 1] Determine if Zombie is Walker/Runner/Sprinter
  ;;[1 1 1] Set Total Zombie Runners. Check if Round is over 20 for Sprinters
  (Variables|Default|SetTotal%20Runners%20In%20Round (Math|Conversions|ToFloat(Integer) (Math|Float|Round (* (Variables|Default|GetTotalEnemyInRound) (/ (Variables|Default|GetRound) 2e+01)))))
  (if (< _round 2e+01)
    (Variables|Default|SetTotal%20Sprinters%20In%20Round 0.0)
    (else
      (Variables|Default|SetTotal%20Sprinters%20In%20Round (Math|Conversions|ToFloat(Integer) (Math|Float|Round (* (- _round 19.0) 2.0))))))
  (if (< (Variables|Default|GetRound) 4.0)
    ;;[1 1 1] Set all zombies to walkers
    (Variables|Default|SetZombie%20Max%20Walk%20Speed (Variables|Default|GetWalk%20Speed))
    (else
      ;;[1 1 1] Check if all Runners for the round are spawned in. If Runner can spawn, chance to spawn runner
      (if (< (Variables|Default|GetRunnersSpawned) (Variables|Default|GetTotal%20Runners%20In%20Round))
        ;;[1 1 1] Set to Runner and increment runners spawn
        (if (<= (Math|Random|RandomFloatinRange 0.0 1.0) (/ (- (Variables|Default|GetTotal%20Runners%20In%20Round) (Variables|Default|GetRunnersSpawned)) (- (Variables|Default|GetTotalEnemyInRound) (Variables|Default|GetZombiesSpawned))))
          (Variables|Default|SetZombie%20Max%20Walk%20Speed (Variables|Default|GetRun%20Speed))
          (Variables|Default|SetRunnersSpawned (+ (Variables|Default|GetRunnersSpawned) 1.0))
          (if (and (< (Variables|Default|GetSprintersSpawned) (Variables|Default|GetTotal%20Sprinters%20In%20Round)) (> (Variables|Default|GetRound) 19.0))
            ;;[1 1 1] Chance to spawn sprinter from runner count, taking away from runner and sprinter count
            (if (<= (Math|Random|RandomFloatinRange 0.0 1.0) (/ (- (Variables|Default|GetTotal%20Sprinters%20In%20Round) (Variables|Default|GetSprintersSpawned)) (- (Variables|Default|GetTotalEnemyInRound) (Variables|Default|GetZombiesSpawned))))
              (Variables|Default|SetZombie%20Max%20Walk%20Speed (Variables|Default|GetSprint%20Speed))
              (Variables|Default|SetSprintersSpawned (+ (Variables|Default|GetSprintersSpawned) 1.0))
              (Variables|Default|SetRunnersSpawned (- (Variables|Default|GetRunnersSpawned) 1.0))))
          (else
            ;;[1 1 1] Set to Walker if chances fail
            (Variables|Default|SetZombie%20Max%20Walk%20Speed (Variables|Default|GetWalk%20Speed) :!label _label)))
        (else
          (goto _label))))))

(fn AddPoints
  (params (Amount :type Float%20%28double-precision%29))
  ;[1 1 1] Add player points and play animation to screen
  (Variables|Default|SetPoints (+ Amount (Variables|Default|GetPoints)))
  (bind _returnvalue (UserInterface|CreateWidget "/Game/_Project/UI/PointsToChange_W.PointsToChange_W_C" 0 (Utilities|Text|FormatText "+{Amount}" Amount)))
  (UserInterface|Viewport|AddtoViewport _returnvalue 0))

(fn RemovePoints
  (params (Amount :type Float%20%28double-precision%29))
  ;[1 1 1] Remove player points and play animation to screen
  (Variables|Default|SetPoints (- (Variables|Default|GetPoints) Amount))
  (bind _returnvalue (UserInterface|CreateWidget "/Game/_Project/UI/PointsToChangeNegative_W.PointsToChangeNegative_W_C" 0 (Utilities|Text|FormatText "-{Amount}" Amount)))
  (UserInterface|Viewport|AddtoViewport _returnvalue 0))