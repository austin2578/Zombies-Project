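; BP_Zombie_1 is an enemy zombie that deals melee swipe damage to the player, BP_Vivian.
; Overlaps on its left and right hand hitboxes run duplicate logic that removes health through Vivian's HealthComponent, halts restoration and plays a hit sound.
; The CanDamage flag gates both hands and is cleared on a hit, limiting damage to once per swing.
; A lethal hit triggers Vivian's death, otherwise health restoration is scheduled.
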(event OnComponentBeginOverlap(RightHandHitbox)
  (params (OverlappedComponent :type Primitive%20Component%20Object%20Reference) (OtherActor :type Actor%20Object%20Reference) (OtherComp :type Primitive%20Component%20Object%20Reference) (OtherBodyIndex :type Integer) (bFromSweep :type Boolean) (SweepResult :type Hit%20Result%20Structure%20%28by%20ref%29))
  ;[1 1 1] Left and Right Hand Swipe
  ;[1 1 1] Check if zombie can damage
  (if (Variables|Default|GetCanDamage?)
    ;[1 1 1] Remove Player Health and Play Hit Sound
    (bind _asbp_vivian (Utilities|Casting|CastToBP_Vivian OtherActor))
    (bind _dead_ (Default|HealthRemove (Variables|/Game/MetaHumans/Vivian/BP_Vivian.BP_Vivian_C|GetHealth%20Component _asbp_vivian) 5e+01 self))
    (Variables|/Game/_Project/Components/BPC_Health.BPC_Health_C|SetHealth%20Restoring? (Variables|/Game/MetaHumans/Vivian/BP_Vivian.BP_Vivian_C|GetHealth%20Component _asbp_vivian) false)
    (Audio|PlaySound2D "/Game/_Project/Resources/Audio/BodyshotCue.BodyshotCue" 1.0 1.0 0.0 0 0)
    ;[1 1 1] Commence Death if player is dead, if alive start restoring Health. Zombie can no longer apply damage during swing
    (if _dead_
      (Default|Death _asbp_vivian)
      (Variables|Default|SetCanDamage? false)
      (else
        (Variables|Default|SetCanDamage? false)
        (Default|SetRestoreHealth _asbp_vivian)))))

(event OnComponentBeginOverlap(LeftHandHitbox)
  (params (OverlappedComponent :type Primitive%20Component%20Object%20Reference) (OtherActor :type Actor%20Object%20Reference) (OtherComp :type Primitive%20Component%20Object%20Reference) (OtherBodyIndex :type Integer) (bFromSweep :type Boolean) (SweepResult :type Hit%20Result%20Structure%20%28by%20ref%29))
  ;[1 1 1] Left and Right Hand Swipe
  (if (Variables|Default|GetCanDamage?)
    ;[1 1 1] Remove Player Health and Play Hit Sound
    (bind _asbp_vivian (Utilities|Casting|CastToBP_Vivian OtherActor))
    (bind _dead_ (Default|HealthRemove (Variables|/Game/MetaHumans/Vivian/BP_Vivian.BP_Vivian_C|GetHealth%20Component _asbp_vivian) 5e+01 self))
    (Variables|/Game/_Project/Components/BPC_Health.BPC_Health_C|SetHealth%20Restoring? (Variables|/Game/MetaHumans/Vivian/BP_Vivian.BP_Vivian_C|GetHealth%20Component _asbp_vivian) false)
    (Audio|PlaySound2D "/Game/_Project/Resources/Audio/BodyshotCue.BodyshotCue" 1.0 1.0 0.0 0 0)
    ;[1 1 1] Commence Death if player is dead, if alive start restoring Health. Zombie can no longer apply damage during swing
    (if _dead_
      (Default|Death _asbp_vivian)
      (Variables|Default|SetCanDamage? false)
      (else
        (Variables|Default|SetCanDamage? false)
        (Default|SetRestoreHealth _asbp_vivian)))))

(event EventBeginPlay
  (|CallParentFunction))

(event Collision|EventActorBeginOverlap
  (params (OtherActor :type Actor%20Object%20Reference))
  (|CallParentFunction OtherActor) ; This node is disabled and will not be called.\nDrag off pins to build functionality.
)

(event EventTick
  (params (DeltaSeconds :type Float%20%28single-precision%29))
  (|CallParentFunction DeltaSeconds) ; This node is disabled and will not be called.\nDrag off pins to build functionality.
)

(fn ConstructionScript
  (|CallParentFunction))