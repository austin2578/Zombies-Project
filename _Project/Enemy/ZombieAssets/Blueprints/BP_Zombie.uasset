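; Zombie enemy character for a wave-based mode, with configurable max speed and health.
; Damage shows hit markers and awards points, with a stab bonus on kills; death unpossesses the AI, disables collision, plays an animation and decrements the GameMode count that ends the round.
; Tick tracks falling and smoothly yaws attacking zombies toward the player.
; JumpToDestination launches it along a suggested projectile arc to AI smart link destinations.
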(event Custom|Death
  (bind _aszombie_aic (Utilities|Casting|CastToZombie_AIC (AI|GetAIController self)))
  ;[1 1 1] Set as dead, remove AI controller and collision, and disable movement
  (Variables|/Game/_Project/Enemy/AI/Zombie_AIC.Zombie_AIC_C|SetIsDead? _aszombie_aic true)
  (Pawn|UnPossess _aszombie_aic)
  (Pawn|Components|CharacterMovement|DisableMovement (Variables|Character|GetCharacterMovement))
  (Collision|SetCollisionEnabled (Variables|Character|GetMesh) "NoCollision")
  (Collision|SetCollisionEnabled (Variables|Default|GetCapsuleComponent) "NoCollision")
  ;[1 1 1] Play Death Animation
  (Utilities|FlowControl|Delay 0.05)
  (Components|Animation|SetAnimationMode (Variables|Character|GetMesh) "AnimationSingleNode" true)
  (Components|Animation|PlayAnimation (Variables|Character|GetMesh) "/Game/_Project/Enemy/ZombieAssets/Anims/Zombie_Death.Zombie_Death" false)
  ;[1 1 1] Adjust Zombie count and end round if no more zombies in round
  (bind _asgm_zombie_waves (Utilities|Casting|CastToGM_ZombieWaves (Game|GetGameMode)))
  (bind _output_get (Variables|/Game/_Project/GameMode/GM_ZombieWaves.GM_ZombieWaves_C|SetTempZombieKills _asgm_zombie_waves (- (Variables|/Game/_Project/GameMode/GM_ZombieWaves.GM_ZombieWaves_C|GetTempZombieKills _asgm_zombie_waves) 1.0)))
  (if (== _output_get 0.0)
    (Default|CallRoundEnd _asgm_zombie_waves))
  (Utilities|FlowControl|Delay 15.0)
  (Actor|DestroyActor))

(event EventBeginPlay
  ;[1 1 1] Set Max Speed based off Walker/Runner/Sprinter Selection
  (Variables|/Script/Engine.CharacterMovementComponent|SetMaxWalkSpeed (Variables|Character|GetCharacterMovement) (Variables|Default|GetMaxSpeed)))

(event Collision|EventActorBeginOverlap
  (params (OtherActor :type Actor%20Object%20Reference)))

(event EventTick
  (params (DeltaSeconds :type Float%20%28single-precision%29))
  ;[1 1 1] Comment
  ;;[1 1 1] Zombie will always rotate towards player when attacking
  (CallFunction|AttackRotation)
  ;;[1 1 1] Set falling value
  (if (!= (.Z (Math|Vector|BreakVector (Variables|/Script/Engine.MovementComponent|GetVelocity (Variables|Character|GetCharacterMovement)))) 0.0)
    (Variables|Default|SetFalling? true)
    (else
      (Variables|Default|SetFalling? false))))

(event Game|Damage|EventAnyDamage
  (params (Damage :type Float%20%28single-precision%29) (DamageType :type Damage%20Type%20Object%20Reference) (InstigatedBy :type Controller%20Object%20Reference) (DamageCauser :type Actor%20Object%20Reference))
  ;[1 1 1] On damage from player
  ;;[1 1 1] Check if damage will kill zombie
  (if (> (- (Variables|Default|GetHealth) Damage) 0.0)
    ;;[1 1 1] If Alive, adjust health, play hit marker, and award proper points
    (Variables|Default|SetHealth (- (Variables|Default|GetHealth) Damage))
    (bind _foundwidgets (Widget|GetAllWidgetsOfClass "/Game/_Project/UI/PlayerUI_W.PlayerUI_W_C" true))
    (Default|HitMarker (Utilities|Array|Get(acopy) _foundwidgets) false)
    (bind _asgm_zombie_waves (Utilities|Casting|CastToGM_ZombieWaves (Game|GetGameMode)))
    (Default|AddPoints _asgm_zombie_waves 1e+01)
    (else
      ;;[1 1 1] On kill, trigger death sequence, play hitmarker, and award proper points
      (Variables|Default|SetHealth 0.0)
      (CallFunction|Death)
      (bind _foundwidgets_2 (Widget|GetAllWidgetsOfClass "/Game/_Project/UI/PlayerUI_W.PlayerUI_W_C" true))
      (Default|HitMarker (Utilities|Array|Get(acopy) _foundwidgets_2) true)
      (bind _asbp_vivian (Utilities|Casting|CastToBP_Vivian (Game|GetPlayerCharacter 0)))
      ;;;[1 1 1] Check if stabbing for the kill, award proper points for sstab kill
      (if (Variables|/Game/MetaHumans/Vivian/BP_Vivian.BP_Vivian_C|GetIsStabbing? _asbp_vivian)
        (bind _asgm_zombie_waves_2 (Utilities|Casting|CastToGM_ZombieWaves (Game|GetGameMode)))
        (Default|AddPoints _asgm_zombie_waves_2 1.3e+02)
        (else
          (bind _asgm_zombie_waves_3 (Utilities|Casting|CastToGM_ZombieWaves (Game|GetGameMode)))
          (Default|AddPoints _asgm_zombie_waves_3 5e+01)))
      (Variables|Default|SetIsDying? true))))

(fn ConstructionScript
  (|CallParentFunction)
  ;[1 1 1] Set Current Health to Max Health
  (Variables|Default|SetHealth (Variables|Default|GetMaxHealth)))

(fn JumptoDestination
  (params (Destination :type Vector))
  (bind (_x _y _z) (Math|Vector|BreakVector Destination))
  ;[1 1 1] Jump to AI Smart Link Location
  (bind _outlaunchvelocity (Game|SuggestProjectileVelocityCustomArc (Transformation|GetActorLocation) (Math|Vector|MakeVector _x _y (+ _z 2.5e+02)) 0.0 0.5))
  (Character|LaunchCharacter _outlaunchvelocity true true))

(fn AttackRotation
  (bind _capsulecomponent (Variables|Default|GetCapsuleComponent))
  ;[1 1 1] Rotate zombie towards player during attack
  (if (> (Variables|Default|GetHealth) 0.0)
    (if (Variables|Default|GetAttacking?)
      (Transformation|SetWorldRotation (Variables|Default|GetCapsuleComponent) (Math|Rotator|MakeRotator 0.0 0.0 (.yaw (Math|Interpolation|RInterpTo (Transformation|GetWorldRotation _capsulecomponent) (Math|Rotator|FindLookatRotation (Transformation|GetWorldLocation _capsulecomponent) (Transformation|GetWorldLocation (Variables|/Script/Engine.Character|GetMesh (Game|GetPlayerCharacter 0)))) (Utilities|Time|GetWorldDeltaSeconds) 5.0))) false false))))