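; A health component that handles damage and healing for the player.
; HealthRemove stops health restoring, subtracts damage clamped between zero and max, and returns whether health has reached zero.
; It finds the PlayerUI_W widget by class and plays its on-hit feedback with the attacker reference.
; HealthAdd applies clamped healing; the event graph is unused.
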(event EventBeginPlay)

(event EventTick
  (params (DeltaSeconds :type Float%20%28single-precision%29)))

(fn HealthRemove
  (params (Amount :type Float%20%28double-precision%29) (EnemyRef :type Actor%20Object%20Reference))
  ;[1 1 1] Removes from Health Current for Player and Plays On Hit Animation. If Player health reaches 0 they die
  (Variables|Default|SetHealth%20Restoring? false)
  (bind _output_get (Variables|Default|SetHealth%20Current (Math|Float|Clamp(Float) (- (Variables|Default|GetHealth%20Current) Amount) 0.0 (Variables|Default|GetHealth%20Max))))
  (bind _foundwidgets (Widget|GetAllWidgetsOfClass "/Game/_Project/UI/PlayerUI_W.PlayerUI_W_C" true))
  (Default|OnHit (Utilities|Array|Get(acopy) _foundwidgets) EnemyRef)
  (if (<= _output_get 0.0)
    (return true)
    (else
      (return false))))

(fn HealthAdd
  (params (Amount :type Float%20%28double-precision%29))
  (Variables|Default|SetHealth%20Current (Math|Float|Clamp(Float) (+ (Variables|Default|GetHealth%20Current) Amount) 0.0 (Variables|Default|GetHealth%20Max))))